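; Robot Blueprint that takes player input for switching tasks and grabbing with either hand.
; Number keys 1 to 3 set CurrentJerarquiaTask to the assemble (Armar), rotation or play task.
; GrabRight and GrabLeft input actions forward press and release to grab functions not defined in this Blueprint.
; SelectPressed and SelectReleased calls are left unwired, and the construction script is empty.
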(event EventBeginPlay)

(event Collision|EventActorBeginOverlap
  (params (OtherActor :type Actor%20Object%20Reference)))

(event EventTick
  (params (DeltaSeconds :type Float%20%28single-precision%29)))

(event Input|ActionEvents|InputActionGrabRight
  (params (Key :type Key%20Structure))
  (:Pressed
    (Class|Robot|GrabRightPressed))
  (:Released
    (Class|Robot|GrabRightReleased)))

(event Input|ActionEvents|InputActionSeleccionar
  (params (Key :type Key%20Structure)))

(event Input|ActionEvents|InputActionGrabLeft
  (params (Key :type Key%20Structure))
  (:Pressed
    (Class|Robot|GrabLeftPressed))
  (:Released
    (Class|Robot|GrabLeftReleased)))

(event Input|KeyboardEvents|1
  (params (Key :type Key%20Structure))
  (:Pressed
    (Variables|Default|SetCurrentJerarquiaTask "EArmarTask")))

(event Input|KeyboardEvents|2
  (params (Key :type Key%20Structure))
  (:Pressed
    (Variables|Default|SetCurrentJerarquiaTask "ERotationTask")))

(event Input|KeyboardEvents|3
  (params (Key :type Key%20Structure))
  (:Pressed
    (Variables|Default|SetCurrentJerarquiaTask "EPlayTask")))

(fn ConstructionScript)