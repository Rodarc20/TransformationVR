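; Nodo_BP is a node Blueprint in the transformation hierarchy that displays a part's name, translation and rotation through a widget component.
; On Tick, once IdParte is not -1, it casts the component's user widget to NodoWidget and passes it the three values.
; The Actualizado flag limits this to one successful update, so Tick serves as a deferred initializer while BeginPlay stays empty.
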(event EventBeginPlay)

(event Collision|EventActorBeginOverlap
  (params (OtherActor :type Actor%20Object%20Reference)))

(event EventTick
  (params (DeltaSeconds :type Float%20%28single-precision%29))
  (if (not (Variables|Default|GetbActualizado))
    (if (!= (Variables|Default|GetIdParte) -1)
      (bind _asnodo_widget (Utilities|Casting|CastToNodoWidget (UserInterface|GetUserWidgetObject (Variables|Default|GetWidget))))
      (Default|CambiarParte _asnodo_widget (Variables|Default|GetNombreParte))
      (Default|IngresarTraslacion _asnodo_widget (Variables|Default|GetTextoTraslacion))
      (Default|IngresarRotacion _asnodo_widget (Variables|Default|GetTextoRotacion))
      (Variables|Default|SetbActualizado true))))

(fn ConstructionScript)